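; GridManager is an actor that builds a grid of GridCell actors at BeginPlay.
; PopulateGrid clears GridArray, then loops over GridSize X and Y, spawning a cell at each GridSpacing step and storing it in the array.
; Positions are absolute world coordinates at Z zero, shifted by a half-width offset to centre on the origin.
; That offset derives from GridSize.X alone, so only square grids centre on both axes.
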(event `self.ReceiveBeginPlay`
  (`self.PopulateGrid`))

(fn `PopulateGrid`
  (locals (WorldOffset :type "Float (double-precision)"))
  (bind _gridsize_x (`KismetMathLibrary.BreakVector` (`self.gridSize`)))
  (bind _gridspacing (`self.gridSpacing`))
  (bind (_gridsize_x_2 _gridsize_y) (`KismetMathLibrary.BreakVector` (`self.gridSize`)))
  (bind _gridsize_x_3 (`KismetMathLibrary.BreakVector` (`self.gridSize`)))
  (bind _gridspacing_2 (`self.gridSpacing`))
  (bind _returnvalue (`KismetMathLibrary.FTrunc` (`local.WorldOffset`)))
  (`KismetArrayLibrary.Array_Clear` (`self.gridArray`))
  (set `local.WorldOffset` (- (* (* _gridspacing _gridsize_x) 0.5) (* _gridspacing 0.5)))
  ;[1 1 1] Loop for Grid Size X
  (for _index (range (+ (`KismetMathLibrary.Conv_Int64ToInt` (- (`KismetMathLibrary.Round64` _gridsize_x_3) 1)) 1))
    ;[1 1 1] Loop for Grid Size Y
    (for _index_2 (range (+ (`KismetMathLibrary.Conv_Int64ToInt` (- (`KismetMathLibrary.Round64` _gridsize_y) 1)) 1))
      ;[1 1 1] Spawn Actor and Place in Array
      (bind _returnvalue_2 (`|SpawnActorFromClass` "/Game/Blueprints/Grid/GridCell.GridCell_C" (`KismetMathLibrary.MakeTransform` (`KismetMathLibrary.MakeVector` (`KismetMathLibrary.Conv_IntToDouble` (- (* _index _gridspacing_2) _returnvalue)) (`KismetMathLibrary.Conv_IntToDouble` (- (* _index_2 _gridspacing_2) _returnvalue)))) "AlwaysSpawn" "OverrideRootScale" null null))
      (`KismetArrayLibrary.Array_Add` (`self.gridArray`) _returnvalue_2))))

(fn `UserConstructionScript`)
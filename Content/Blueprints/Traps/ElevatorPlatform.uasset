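; Trap elevator platform that shuttles between a top and bottom marker, flipping 180 degrees in pitch at each end.
; MovePlatform chains MoveComponentTo calls on the root, scaling LiftTime by remaining distance to hold a steady speed, then calls itself to loop.
; On the first pass, starting pitch decides whether it heads up or down; InitialSpin then locks in the full cycle.
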(event `MovePlatform`
  (params (Top :type "SceneComponent Object Reference") (Bottom :type "SceneComponent Object Reference"))
  (bind _returnvalue (`SceneComponent.K2_GetComponentLocation` Top))
  (bind _returnvalue_2 (`SceneComponent.K2_GetComponentLocation` Bottom))
  (bind _defaultsceneroot (`self.DefaultSceneRoot`))
  (bind _defaultsceneroot_2 (`self.DefaultSceneRoot`))
  (bind _defaultsceneroot_3 (`self.DefaultSceneRoot`))
  (bind _defaultsceneroot_4 (`self.DefaultSceneRoot`))
  (bind (_relativerotation_roll _relativerotation_pitch _relativerotation_yaw) (`KismetMathLibrary.BreakRotator` (`SceneComponent.RelativeRotation` _defaultsceneroot_4)))
  (bind (_relativerotation_roll_2 _relativerotation_pitch_2 _relativerotation_yaw_2) (`KismetMathLibrary.BreakRotator` (`SceneComponent.RelativeRotation` _defaultsceneroot_2)))
  (bind (_relativerotation_roll_3 _relativerotation_pitch_3) (`KismetMathLibrary.BreakRotator` (`SceneComponent.RelativeRotation` (`self.DefaultSceneRoot`))))
  (set `self.distBetween` (`KismetMathLibrary.Vector_Distance` (`SceneComponent.K2_GetComponentLocation` Top) (`SceneComponent.K2_GetComponentLocation` Bottom)))
  (if (`self.InitialSpin`)
    (`KismetSystemLibrary.MoveComponentTo` _defaultsceneroot _returnvalue (`SceneComponent.RelativeRotation` _defaultsceneroot) false false (* (`self.LiftTime`) (/ (`KismetMathLibrary.Vector_Distance` _returnvalue (`SceneComponent.K2_GetComponentLocation` _defaultsceneroot)) (`self.distBetween`))) :!label _label)
    (`KismetSystemLibrary.MoveComponentTo` _defaultsceneroot_2 (`SceneComponent.RelativeLocation` _defaultsceneroot_2) (`KismetMathLibrary.MakeRotator` _relativerotation_roll_2 (+ _relativerotation_pitch_2 180.0) _relativerotation_yaw_2) false false 2.5)
    (`KismetSystemLibrary.Delay` 0.0)
    (elif (== _relativerotation_pitch_3 0.0)
      (goto _label)
      (else
        _)))
  (`KismetSystemLibrary.MoveComponentTo` _defaultsceneroot_3 _returnvalue_2 (`SceneComponent.RelativeRotation` _defaultsceneroot_3) false false (* (`self.LiftTime`) (/ (`KismetMathLibrary.Vector_Distance` _returnvalue_2 (`SceneComponent.K2_GetComponentLocation` _defaultsceneroot_3)) (`self.distBetween`))))
  (`KismetSystemLibrary.MoveComponentTo` _defaultsceneroot_4 (`SceneComponent.RelativeLocation` _defaultsceneroot_4) (`KismetMathLibrary.MakeRotator` _relativerotation_roll (- _relativerotation_pitch 180.0) _relativerotation_yaw) false false 2.5 true)
  (set `self.InitialSpin` true)
  (`self.MovePlatform` Top Bottom))

(fn `Movement`
  (params (Platform :type "SceneComponent Object Reference")))

(fn `UserConstructionScript`)
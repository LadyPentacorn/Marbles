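; Pusher trap that endlessly slides its Face component out and back along relative X by MoveDist.
; Push, started on BeginPlay, chains timed MoveComponentTo moves and delays, then calls itself to loop.
; Two helper functions compute the forward and back targets from the Face's current relative transform.
; BeginPlay also stretches and offsets the Arm along X once, based on MoveDist.
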(event `Push`
  (bind _face (`self.Face`))
  (`|ExecutionSequence`
    (:`then_0`
      (bind (_newpos _relativerot) (`self.Move Pusher Forward` _face))
      (`KismetSystemLibrary.MoveComponentTo` _face _newpos _relativerot false false 1.5)
      (`KismetSystemLibrary.Delay` 2.0)
      (bind (_newpos_2 _relativerot_2) (`self.Move Pusher Back` _face))
      (`KismetSystemLibrary.MoveComponentTo` _face _newpos_2 _relativerot_2 false false 1.5)
      (`KismetSystemLibrary.Delay` 2.0)
      (`self.Push`))))

(event `self.ReceiveBeginPlay`
  (bind _arm (`self.Arm`))
  (bind _arm_2 (`self.Arm`))
  (bind (_relativelocation_x _relativelocation_y _relativelocation_z) (`KismetMathLibrary.BreakVector` (`SceneComponent.RelativeLocation` _arm)))
  (bind (_relativescale3d_x _relativescale3d_y _relativescale3d_z) (`KismetMathLibrary.BreakVector` (`SceneComponent.RelativeScale3D` _arm_2)))
  (`self.Push`)
  (`SceneComponent.SetRelativeScale3D` _arm_2 (`KismetMathLibrary.MakeVector` (* _relativescale3d_x (/ (`self.MoveDist`) 100.0)) _relativescale3d_y _relativescale3d_z))
  (bind _output_get (set `self.StartX` _relativelocation_x))
  (`KismetSystemLibrary.MoveComponentTo` _arm (`KismetMathLibrary.MakeVector` (- _output_get (/ (- (`self.MoveDist`) _output_get) 2.0)) _relativelocation_y _relativelocation_z) (`SceneComponent.RelativeRotation` _arm)))

(fn `Move Pusher Back`
  (params (Mesh :type "StaticMeshComponent Object Reference"))
  (returns (NewPos :type "Vector Structure") (RelativeRot :type "Rotator Structure"))
  (bind (_relativelocation_x _relativelocation_y _relativelocation_z) (`KismetMathLibrary.BreakVector` (`SceneComponent.RelativeLocation` Mesh)))
  (return (`KismetMathLibrary.MakeVector` (- _relativelocation_x (`self.MoveDist`)) _relativelocation_y _relativelocation_z) (`SceneComponent.RelativeRotation` Mesh)))

(fn `Move Pusher Forward`
  (params (Mesh :type "StaticMeshComponent Object Reference"))
  (returns (NewPos :type "Vector Structure") (RelativeRot :type "Rotator Structure"))
  (bind (_relativelocation_x _relativelocation_y _relativelocation_z) (`KismetMathLibrary.BreakVector` (`SceneComponent.RelativeLocation` Mesh)))
  (return (`KismetMathLibrary.MakeVector` (+ _relativelocation_x (`self.MoveDist`)) _relativelocation_y _relativelocation_z) (`SceneComponent.RelativeRotation` Mesh)))

(fn `UserConstructionScript`)
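; Vent trap that blows marbles along its up direction while they overlap it.
; Begin overlap adds the static mesh component of any actor tagged Marble to an array, and Tick applies PushForce to each entry.
; The end-overlap event passes OverlappedActor rather than OtherActor to RemoveMarble, and the file shows no binding for it, so departing marbles likely stay in the array.
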(event `self.ReceiveBeginPlay`)

(event `self.ReceiveTick`
  (params (DeltaSeconds :type "Float (single-precision)"))
  (`self.PushMarbles`))

(event `self.ReceiveActorBeginOverlap`
  (params (OtherActor :type "Actor Object Reference"))
  (`self.AddMarble` OtherActor))

(event `OnActorEndOverlap_Event_0`
  (params (OverlappedActor :type "Actor Object Reference") (OtherActor :type "Actor Object Reference"))
  (`self.RemoveMarble` OverlappedActor))

(fn `AddMarble`
  (params (MarbleHit :type "Actor Object Reference"))
  (if (`self.ActorHasTag` MarbleHit "Marble")
    (`KismetSystemLibrary.PrintString` "Marble Hit")
    (`KismetArrayLibrary.Array_Add` (`self.Marbles`) (`self.GetComponentByClass` MarbleHit "/Script/Engine.StaticMeshComponent"))))

(fn `PushMarbles`
  (if (> (`KismetArrayLibrary.Array_Length` (`self.Marbles`)) 0)
    (for _array_element (`self.Marbles`)
      (`PrimitiveComponent.AddForce` _array_element (* (`SceneComponent.GetUpVector` (`self.DefaultSceneRoot`)) (`self.PushForce`)) "None" false))))

(fn `RemoveMarble`
  (params (MarbleHit :type "Actor Object Reference"))
  (if (`self.ActorHasTag` MarbleHit "Marble")
    (`KismetArrayLibrary.Array_RemoveItem` (`self.Marbles`) (`self.GetComponentByClass` MarbleHit "/Script/Engine.StaticMeshComponent"))))

(fn `UserConstructionScript`)